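; Test player Blueprint that plays an in-actor cutscene when the 2 key is pressed.
; The key press switches the player camera's view target to the Sequencechild child actor and starts the ActorSequence component.
; It then binds a custom event to the sequence's finish, which returns the view target to this actor.
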(event Custom|CustomEvent
  (Game|Player|SetViewTargetwithBlend (Game|GetPlayerController 0) self 0.0 "VTBlend_EaseInOut" 1.0 false))

(event EventBeginPlay)

(event Collision|EventActorBeginOverlap
  (params (OtherActor :type Actor%20Object%20Reference)))

(event EventTick
  (params (DeltaSeconds :type Float%20%28single-precision%29)))

(event Input|KeyboardEvents|2
  (params (Key :type Key%20Structure :default "None"))
  (bind _actorsequence (Variables|Default|GetActorSequence))
  (bind _sequenceplayer (Variables|/Script/ActorSequence.ActorSequenceComponent|GetSequencePlayer _actorsequence))
  (:Pressed
    (Game|Player|SetViewTargetwithBlend (Game|GetPlayerController 0) (Variables|/Script/Engine.ChildActorComponent|GetChildActor (Variables|Default|Getsequencechild)) 0.0 "VTBlend_EaseInOut" 1.0 false)
    (Sequencer|Player|Play _sequenceplayer :!class /Script/MovieScene.MovieSceneSequencePlayer)
    (EventDispatchers|BindEventtoOnFinished _sequenceplayer (delegate Custom|CustomEvent))))

(fn ConstructionScript)